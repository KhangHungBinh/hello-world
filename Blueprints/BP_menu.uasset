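; BP_menu is a possessable menu pawn that shows the Menu widget while possessed and turns horizontal touch swipes into menu messages.
; Possession creates the widget and adds it to the viewport; unpossession removes it.
; Finger 1 press and release positions are compared on X, with no minimum distance, to call the widget's swipe-right or swipe-left message.
; Swipe-driven yaw and pitch camera code remains but is disconnected.
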(event `self.ReceivePossessed`
  (params (NewController :type "Controller Object Reference"))
  ;[1 1 1] chuyen nhan vat
  (bind _returnvalue (`|CreateWidget` "/Game/Blueprints/Menu.Menu_C"))
  (`UserWidget.AddToViewport` _returnvalue 0)
  (set `self.menu` _returnvalue))

(event `self.ReceiveUnpossessed`
  (params (OldController :type "Controller Object Reference"))
  ;[1 1 1] chuyen nhan vat
  (`Widget.RemoveFromParent` (stale `self.ReceivePossessed` _returnvalue)))

(event `InputAction|Finger 1`
  (params (Key :type "Key Structure"))
  (bind _menu (`self.menu`))
  (bind (_locationx _locationy) (`PlayerController.GetInputTouchState` (`GameplayStatics.GetPlayerController` 0) "Touch1"))
  (bind _returnvalue (- (`KismetMathLibrary.BreakVector2D` (`self.PriorLoc`)) (`KismetMathLibrary.BreakVector2D` (`self.StartLoc`))))
  (bind _returnvalue_2 (`KismetMathLibrary.MakeVector2D` _locationx _locationy))
  ;[1 1 1] Swipe
  (:`Pressed`
    (set `self.StartLoc` _returnvalue_2))
  (:`Released`
    (set `self.PriorLoc` _returnvalue_2)
    (if (> _returnvalue 0.0)
      (`KismetSystemLibrary.RetriggerableDelay` 0.0)
      (message `/Game/Blueprints/pinchzoom.swiperight` _menu)
      (elif (< _returnvalue 0.0)
        (`KismetSystemLibrary.RetriggerableDelay` 0.0)
        (message `/Game/Blueprints/pinchzoom.swipeleft` _menu)))))

(fn `UserConstructionScript`)