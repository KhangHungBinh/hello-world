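; Pawn that shows the Vitri_HUD location-image (AnhViTri) widget while possessed and handles pinch zoom and drag panning on it.
; Gates separate pinching from one-finger dragging, with zoom requests sent to the HUD as messages.
; Panning converts pointer movement to canvas coordinates and clamps the image position by zoom state.
; The Timeline meant to tick this logic has no incoming trigger, and several other fragments are disconnected.
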(event `Key|Gesture_Pinch`
  (params (Key :type "Key Structure"))
  ;[1 1 1] zoom in
  (:`Pressed`
    (`/Engine/EditorBlueprintResources/StandardMacros.Gate` true :!via `Open` :!label _label
      (:`Exit`
        (message `/Game/Blueprints/pinchzoom.FunctionPinchZoomIn` (`self.vitri_HUD`) 0.5)
        (set `self.in` true))))
  (:`Released`
    (goto _label :!via `Close`)))

(event `InputAxis|Pinch Touch`
  (params (AxisValue :type "Float (single-precision)")))

(event `Key|Gesture_Pinch`
  (params (Key :type "Key Structure"))
  (bind (_x _y) (`KismetMathLibrary.BreakVector2D` (`self.image position`)))
  ;[1 1 1] zoom out
  (:`Pressed`
    (`/Engine/EditorBlueprintResources/StandardMacros.Gate` true :!via `Open` :!label _label_2
      (:`Exit`
        (message `/Game/Blueprints/pinchzoom.FunctionPinchZoomOut` (`self.vitri_HUD`) 1.0)
        (set `self.in` false)
        (`CanvasPanelSlot.SetPosition` (`WidgetLayoutLibrary.SlotAsCanvasSlot` (stale `self.ReceivePossessed` _output_get)) (`KismetMathLibrary.MakeVector2D` (`KismetMathLibrary.FClamp` _x -1632.0 -1024.0) (`KismetMathLibrary.FClamp` _y -480.0 -480.0))))))
  (:`Released`
    (goto _label_2 :!via `Close`)))

(event `MouseIsOver`
  (bind (_returnvalue_x _returnvalue_y) (`KismetMathLibrary.BreakVector2D` (`WidgetLayoutLibrary.GetViewportSize`)))
  (bind (_x _y) (`KismetMathLibrary.BreakVector2D` (`self.image position`)))
  (bind (_locationx _locationy) (`PlayerController.GetMousePosition` (`GameplayStatics.GetPlayerController` 0)))
  (bind (_x_2 _y_2) (`KismetMathLibrary.BreakVector2D` (`self.image position`)))
  (bind _returnvalue (`KismetMathLibrary.MakeVector2D` (* _locationx (/ (`self.canvas_x`) _returnvalue_x)) (* _locationy (/ (`self.canvas_y`) _returnvalue_y))))
  ;[1 1 1] Mouse over image
  (set `self.mouseposition_0` _returnvalue)
  (set `self.image position_1` (`CanvasPanelSlot.GetPosition` (`WidgetLayoutLibrary.SlotAsCanvasSlot` (`self.AnhViTri`))))
  (`/Engine/EditorBlueprintResources/StandardMacros.Gate` true :!via `Open`
    (:`Exit`
      ;[1 1 1] zooming or dragging?
      (if (`self.Drag`)
        ;[1 1 1] Move image
        (`/Engine/EditorBlueprintResources/StandardMacros.Gate` true :!label _label_3
          (:`Exit`
            (set `self.image position` (+ (`self.image position_1`) (- _returnvalue (`self.mouseposition_0`))))
            (if (`self.in`)
              (bind _returnvalue_2 (`WidgetLayoutLibrary.SlotAsCanvasSlot` (stale `self.ReceivePossessed` _output_get)))
              ;;[1 1 1] scale 0.5
              (`CanvasPanelSlot.SetPosition` _returnvalue_2 (`KismetMathLibrary.MakeVector2D` (`KismetMathLibrary.FClamp` _x -1632.0 -1024.0) (`KismetMathLibrary.FClamp` _y -480.0 -480.0)))
              (else
                ;;[0.464 0.1676 1] scale 1
                (`CanvasPanelSlot.SetPosition` _returnvalue_2 (`KismetMathLibrary.MakeVector2D` (`KismetMathLibrary.FClamp` _x_2 -2650.0 0.0) (`KismetMathLibrary.FClamp` _y_2 -970.0 0.0)))))))
        (else
          (if (> (stale `InputAxis|Pinch Touch` AxisValue) 1.0)
            (goto _label)
            (else
              (goto _label_2))))))))

(event `Key|Gesture_Pinch`
  (params (Key :type "Key Structure"))
  ;[1 1 1] set condition
  (:`Pressed`
    (set `self.Drag` false))
  (:`Released`
    (set `self.Drag` true)))

(event `MouseIsNotOver`
  ;[1 1 1] Mouse over image
)

(event `self.ReceivePossessed`
  (params (NewController :type "Controller Object Reference"))
  ;[1 1 1] create UI
  (`/Engine/EditorBlueprintResources/StandardMacros.IsValid` (stale `self.ReceivePossessed` _returnvalue)
    (:`Is Valid`
      _)
    (:`Is Not Valid`
      (bind _returnvalue (`|CreateWidget` "/Game/Blueprints/Vitri_HUD.Vitri_HUD_C"))))
  (`UserWidget.AddToViewport` _returnvalue 0)
  (set `self.vitri_HUD` _returnvalue)
  (bind _output_get (set `self.AnhViTri` (`/Game/Blueprints/Vitri_HUD.Anh_ViTri` _returnvalue))))

(event `self.ReceiveUnpossessed`
  (params (OldController :type "Controller Object Reference"))
  ;[1 1 1] create UI
  (`Widget.RemoveFromParent` (stale `self.ReceivePossessed` _returnvalue)))

(event `InputAction|Finger 1`
  (params (Key :type "Key Structure"))
  (bind (_returnvalue_x _returnvalue_y) (`KismetMathLibrary.BreakVector2D` (`WidgetLayoutLibrary.GetViewportSize`)))
  (bind (_locationx _locationy) (`PlayerController.GetMousePosition` (`GameplayStatics.GetPlayerController` 0)))
  ;[1 1 1] Move image
  (:`Pressed`
    (set `self.mouseposition_0` (`KismetMathLibrary.MakeVector2D` (* _locationx (/ (`self.canvas_x`) _returnvalue_x)) (* _locationy (/ (`self.canvas_y`) _returnvalue_y))))
    (set `self.image position_1` (`CanvasPanelSlot.GetPosition` (`WidgetLayoutLibrary.SlotAsCanvasSlot` (`self.AnhViTri`))))
    (goto _label_3 :!via `Open`))
  (:`Released`
    (goto _label_3 :!via `Close`)))

(event `/Game/Blueprints/pinchzoom.DragStart`
  (params (Drag :type Boolean))
  ;[1 1 1] bug can not fix
  (set `self.Drag` Drag))

(event `/Game/Blueprints/pinchzoom.DragRelease`
  (params (Drag :type Boolean))
  ;[1 1 1] bug can not fix
  (set `self.Drag` Drag))

(fn `UserConstructionScript`)